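; Day-night cycle actor that drives the sun, sky, game clock and random rain.
; Tick advances the hour from the configured day length, pitches the Sun and updates the Skydome, scaled by a speed multiplier polled from BtnSpeedUp_BP every frame.
; Clock converts elapsed hours into hours, minutes and a time string.
; A per-tick random roll against the current hour starts rain, which stops after a random, speed-scaled delay.
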(event OnComponentActivated(Rain)
  (params (Component :type Actor%20Component%20Object%20Reference) (bReset :type Boolean))
  ;[0 0 0] Rain
  (Variables|Default|SetRaining true)
  (Utilities|FlowControl|Delay (/ (Math|Random|RandomFloatinRange 3e+01 1.2e+02) (Variables|Default|GetSpeedMultiplier)))
  (Components|Activation|Deactivate Component))

(event OnComponentDeactivated(Rain)
  (params (Component :type Actor%20Component%20Object%20Reference))
  ;[0 0 0] Rain
  (Variables|Default|SetRaining false))

(event EventBeginPlay
  (bind _output_get (Variables|Default|SetOneDay (* (Variables|Default|GetDayLengthInMinutes) 6e+01)))
  (Variables|Default|SetOneHour (/ _output_get 24.0)))

(event Collision|EventActorBeginOverlap
  (params (OtherActor :type Actor%20Object%20Reference)))

(event EventTick
  (params (DeltaSeconds :type Float%20%28single-precision%29))
  (Utilities|FlowControl|Sequence
    (:then_0
      (bind _output_get (Variables|Default|SetHour (+ (Variables|Default|GetHour) (/ DeltaSeconds (/ (Variables|Default|GetOneHour) (Variables|Default|GetSpeedMultiplier))))))
      (bind _output_get_2 (Variables|Default|SetSunAngle (+ (* (/ _output_get 6.0) 9e+01) 9e+01)))
      (Transformation|SetActorRotation (Variables|Default|GetSun) (Math|Rotator|MakeRotator 0.0 _output_get_2 0.0))
      (Default|UpdateSunDirection (Variables|Default|GetSkydome)))
    (:then_1
      (bind _outactors (Actor|GetAllActorsOfClass "/Game/Inventory/btnSpeedUp_BP.btnSpeedUp_BP_C"))
      (bind _output_get_3 (Variables|Default|Setspeed%20up%20btn (Utilities|Array|Get(acopy) _outactors)))
      (Variables|Default|SetSpeedMultiplier (Variables|/Game/Inventory/btnSpeedUp_BP.btnSpeedUp_BP_C|GetSpeedMuliplier _output_get_3)))
    (:then_2
      (CallFunction|Clock))
    (:then_3
      ;[0 0 0] Rain
      (Math|Integer|CompareInt (Variables|Default|GetHours) (Math|Random|RandomInteger 23)
        (:==
          (if (not (Variables|Default|GetRaining))
            (Components|Activation|ToggleActive (Variables|Default|GetRain))))))))

(fn ConstructionScript)

(fn Clock
  (bind _hour (Variables|Default|GetHour))
  (bind _returnvalue (* _hour 6e+01))
  (bind (_remainder _returnvalue_2) (Math|Float|Division(WholeandRemainder) _returnvalue 6e+01))
  (Variables|Default|SetMinutes (Math|Float|Floor _remainder))
  (Variables|Default|SetHours (Math|Float|Floor (.Remainder (Math|Float|Division(WholeandRemainder) (Math|Conversions|ToFloat(Integer) _returnvalue_2) 24.0))))
  (Variables|Default|SetGameTime (Utilities|Array|MakeArray (Variables|Default|GetMinutes) (Variables|Default|GetHours)))
  (bind _output_get (Variables|Default|SetGameTimeString (Utilities|String|BuildString(Integer) (Utilities|String|ToString(Integer) (Utilities|Array|Get(acopy) (Variables|Default|GetGameTime) 1)) ":" (Utilities|Array|Get(acopy) (Variables|Default|GetGameTime))))))