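; Ground actor that changes its mesh material to match the rain and winter flags of the level's DayNight_Blueprint.
; Every Tick checks both flags independently, switching to a puddle material for rain and back to plain ground after short delays when either is false.
; In winter it recreates a snow dynamic material each Tick at zero amount, and a delayed SnowFall event drives that amount through a Timeline.
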(event Custom|Snow%20Fall
  ;[0 0 0] Snow
  (bind _snow_amount (Timeline|Timeline_0 Play)
    (:Update
      (Rendering|Material|SetScalarParameterValue (stale EventTick _returnvalue) "Snow Amount" _snow_amount :!class /Script/Engine.MaterialInstanceDynamic))))

(event EventBeginPlay
  (bind _outactors (Actor|GetAllActorsOfClass "/Game/Assets/Blueprints/DayNight_Blueprint.DayNight_Blueprint_C"))
  (Variables|Default|SetDayNight (Utilities|Array|Get(acopy) _outactors)))

(event Collision|EventActorBeginOverlap
  (params (OtherActor :type Actor%20Object%20Reference)))

(event EventTick
  (params (DeltaSeconds :type Float%20%28single-precision%29))
  (Utilities|FlowControl|Sequence
    (:then_0
      ;[0 0 0] Rain
      (if (Variables|/Game/Assets/Blueprints/DayNight_Blueprint.DayNight_Blueprint_C|GetRaining (Variables|Default|GetDayNight))
        (Utilities|FlowControl|Delay 0.5)
        (Rendering|Material|SetMaterial (Variables|Debug|GetStaticMeshComponent) 0 "/Game/Weather/Rain/Puddles/Puddles_M_Inst.Puddles_M_Inst")
        (else
          (Utilities|FlowControl|Delay 0.5)
          (Rendering|Material|SetMaterial (Variables|Debug|GetStaticMeshComponent) 0 "/Game/Materials/Ground.Ground"))))
    (:then_1
      ;[0 0 0] Snow
      (if (Variables|/Game/Assets/Blueprints/DayNight_Blueprint.DayNight_Blueprint_C|GetWinter (Variables|Default|GetDayNight))
        (bind _returnvalue (Rendering|Material|CreateDynamicMaterialInstance (Variables|/Script/Engine.StaticMeshActor|GetStaticMeshComponent self) 0 "/Game/Weather/Snow/SnowGather_M.SnowGather_M" "None" :!class /Script/Engine.PrimitiveComponent))
        (Rendering|Material|SetScalarParameterValue _returnvalue "Snow Amount" 0.0 :!class /Script/Engine.MaterialInstanceDynamic)
        (Utilities|FlowControl|Delay 1e+01)
        (CallFunction|SnowFall)
        (else
          (Utilities|FlowControl|Delay 0.5)
          (Rendering|Material|SetMaterial (Variables|Debug|GetStaticMeshComponent) 0 "/Game/Materials/Ground.Ground"))))))

(fn ConstructionScript)