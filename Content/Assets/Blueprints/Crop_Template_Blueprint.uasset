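; Crop template actor that grows through three mesh stages and can then be picked up with a VR motion controller.
; BeginPlay swaps the Crop mesh on a timed delay, setting Grabbable from the final mesh swap's return value.
; Pickup and Drop, when Grabbable, toggle physics and attach to or detach from the controller child's Items socket.
; BeginPlay also looks up speed-up button actors but leaves the result unused.
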(event EventBeginPlay
  (Utilities|FlowControl|Sequence
    (:then_0
      (Components|StaticMesh|SetStaticMesh (Variables|Default|GetCrop) (Variables|Default|GetStage1))
      (Utilities|FlowControl|Delay (Variables|Default|GetTimeBetweenStages))
      (Components|StaticMesh|SetStaticMesh (Variables|Default|GetCrop) (Variables|Default|GetStage2))
      (Utilities|FlowControl|Delay (Variables|Default|GetTimeBetweenStages))
      (bind _returnvalue (Components|StaticMesh|SetStaticMesh (Variables|Default|GetCrop) (Variables|Default|GetStage3)))
      (Variables|Default|SetGrabbable _returnvalue))
    (:then_1
      (Actor|GetAllActorsOfClass "/Game/Inventory/btnSpeedUp_BP.btnSpeedUp_BP_C"))))

(event Collision|EventActorBeginOverlap
  (params (OtherActor :type Actor%20Object%20Reference)))

(event EventTick
  (params (DeltaSeconds :type Float%20%28single-precision%29)))

(event EventPickup
  (params (AttachTo :type Scene%20Component%20Object%20Reference))
  (if (Variables|Default|GetGrabbable)
    (bind _asmotion_controller_component (Utilities|Casting|CastToMotionControllerComponent AttachTo))
    (Physics|SetSimulatePhysics (Variables|Default|GetCrop) false)
    (Transformation|AttachComponentToComponent (VehicleSound|GetRootComponent) (Components|GetChildComponent _asmotion_controller_component 0) "Items" "SnapToTarget" "SnapToTarget" "KeepWorld" false)))

(event EventDrop
  (if (Variables|Default|GetGrabbable)
    (Physics|SetSimulatePhysics (Variables|Default|GetCrop) true)
    (Transformation|DetachFromActor "KeepWorld" "KeepWorld" "KeepWorld")))

(fn ConstructionScript)