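; Crop actor that grows through three mesh stages and becomes grabbable by BP_MotionController once fully grown.
; BeginPlay scales stage time by the DayNight season, then chains delayed mesh swaps with growth particles and audio.
; Tick fetches the speed multiplier from BtnSpeedUp_BP via an actor search every frame, dividing stage times by it.
; Tick also tracks elapsed growth against both stages, destroying the spawned progress bar when it completes.
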(event EventBeginPlay
  (bind _p_cropgrowth (Variables|Default|GetP_CropGrowth))
  (bind _p_cropgrowth_2 (Variables|Default|GetP_CropGrowth))
  (bind _p_cropgrowth_3 (Variables|Default|GetP_CropGrowth))
  (Utilities|FlowControl|Sequence
    (:then_0
      ;[0 0 0] Activate particles on crop change
      (Components|Activation|Activate _p_cropgrowth_2 false)
      (Utilities|FlowControl|Delay 1.5)
      (Components|Activation|Deactivate _p_cropgrowth_2))
    (:then_1
      ;[0 0 0] Season change
      (bind _outactors (Actor|GetAllActorsOfClass "/Game/Assets/Blueprints/DayNight_Blueprint.DayNight_Blueprint_C"))
      (Variables|Default|SetDayNight (Utilities|Array|Get(acopy) _outactors))
      (if (Variables|/Game/Assets/Blueprints/DayNight_Blueprint.DayNight_Blueprint_C|GetSpring (Variables|Default|GetDayNight))
        (Variables|Default|SetTimeBetweenStages (/ (Variables|Default|GetTimeBetweenStages) 2.0))
        (elif (Variables|/Game/Assets/Blueprints/DayNight_Blueprint.DayNight_Blueprint_C|GetSummer (Variables|Default|GetDayNight))
          (Variables|Default|SetTimeBetweenStages (* (Variables|Default|GetTimeBetweenStages) 1.0))
          (elif (Variables|/Game/Assets/Blueprints/DayNight_Blueprint.DayNight_Blueprint_C|GetAutum (Variables|Default|GetDayNight))
            (Variables|Default|SetTimeBetweenStages (* (Variables|Default|GetTimeBetweenStages) 2.0))
            (elif (Variables|/Game/Assets/Blueprints/DayNight_Blueprint.DayNight_Blueprint_C|GetWinter (Variables|Default|GetDayNight))
              (Variables|Default|SetTimeBetweenStages (* (Variables|Default|GetTimeBetweenStages) 2.0)))))))
    (:then_2
      ;[0 0 0] Crop stage change
      (Components|StaticMesh|SetStaticMesh (Variables|Debug|GetStaticMeshComponent) (Variables|Default|GetStage1))
      (Utilities|FlowControl|Delay (/ (Variables|Default|GetTimeBetweenStages) (Variables|Default|Getmultipler)))
      (Utilities|FlowControl|Sequence
        (:then_0
          (Components|Activation|Activate _p_cropgrowth_3 false)
          (Utilities|FlowControl|Delay 1.5)
          (Components|Activation|Deactivate _p_cropgrowth_3))
        (:then_1
          (Components|StaticMesh|SetStaticMesh (Variables|Debug|GetStaticMeshComponent) (Variables|Default|GetStage2))
          (Utilities|FlowControl|Delay (/ (Variables|Default|GetTimeBetweenStages) (Variables|Default|Getmultipler)))
          (Utilities|FlowControl|Sequence
            (:then_0
              (Components|Activation|Activate _p_cropgrowth false)
              (Utilities|FlowControl|Delay 1.5)
              (Components|Activation|Deactivate _p_cropgrowth))
            (:then_1
              (bind _returnvalue (Components|StaticMesh|SetStaticMesh (Variables|Debug|GetStaticMeshComponent) (Variables|Default|GetStage3)))
              (Variables|Default|SetGrabbable _returnvalue))
            (:then_2
              (Audio|Components|Audio|Play (Variables|Default|GetCropChange_Audio) 0.0))))
        (:then_2
          (Audio|Components|Audio|Play (Variables|Default|GetCropChange_Audio) 0.0))))
    (:then_3
      (bind _returnvalue_2 (Game|SpawnActorfromClass "/Game/Assets/Blueprints/CropProgressBar_BP.CropProgressBar_BP_C" (Transformation|GetWorldTransform (Variables|Default|GetSpawnPosition)) "Undefined" 0 0))
      (Variables|Default|SetProgressbarActor _returnvalue_2)
      (Variables|Default|Setprogress 0.0))))

(event EventTick
  (params (DeltaSeconds :type Float%20%28single-precision%29))
  ;[0 0 0] Updates Progress Bar
  (Utilities|FlowControl|Sequence
    (:then_0
      (bind _outactors (Actor|GetAllActorsOfClass "/Game/Inventory/btnSpeedUp_BP.btnSpeedUp_BP_C"))
      (bind _output_get (Variables|Default|Setbtnspeedup (Utilities|Array|Get(acopy) _outactors)))
      (Variables|Default|Setmultipler (Variables|/Game/Inventory/btnSpeedUp_BP.btnSpeedUp_BP_C|GetSpeedMuliplier _output_get)))
    (:then_1
      (Variables|Default|SetprogressBarTime (+ (/ (Variables|Default|GetTimeBetweenStages) (Variables|Default|Getmultipler)) (/ (Variables|Default|GetTimeBetweenStages) (Variables|Default|Getmultipler)))))
    (:then_2
      (bind _output_get_2 (Variables|Default|SettimeElapsed (+ DeltaSeconds (Variables|Default|GettimeElapsed))))
      (bind _output_get_3 (Variables|Default|Setprogress (/ _output_get_2 (Variables|Default|GetprogressBarTime))))
      (Math|Float|CompareFloat _output_get_3 1.0
        (:>
          (Utilities|FlowControl|DoOnce false
            (:Completed
              (Actor|DestroyActor (Variables|Default|GetProgressbarActor)))))))))

(event EventPickup
  (params (AttachTo :type Scene%20Component%20Object%20Reference))
  ;[0 0 0] Pick up and drop
  (if (Variables|Default|GetGrabbable)
    (Physics|SetSimulatePhysics (Variables|Debug|GetStaticMeshComponent) false)
    (Transformation|AttachComponentToComponent (VehicleSound|GetRootComponent) AttachTo "None" "SnapToTarget" "SnapToTarget" "KeepWorld" false)))

(event EventDrop
  ;[0 0 0] Pick up and drop
  (if (Variables|Default|GetGrabbable)
    (Physics|SetSimulatePhysics (Variables|Debug|GetStaticMeshComponent) true)
    (Transformation|DetachFromActor "KeepWorld" "KeepWorld" "KeepWorld")))

(fn ConstructionScript)