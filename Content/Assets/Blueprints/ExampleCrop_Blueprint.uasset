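; ExampleCrop is an example crop Blueprint that grows through visual stages on a timer.
; On BeginPlay it sets its static mesh to the first stage, then swaps through the second and third stages to the final crop mesh.
; A latent Delay of the same Growtime separates each swap, so growth runs once without Tick.
; Overlap, Tick and the construction script have no logic.
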(event EventBeginPlay
  (Variables|Default|SetStaticMesh (Variables|Default|GetStage1))
  (Utilities|FlowControl|Delay (Variables|Default|GetGrowtime))
  (Variables|Default|SetStaticMesh (Variables|Default|GetStage2))
  (Utilities|FlowControl|Delay (Variables|Default|GetGrowtime))
  (Variables|Default|SetStaticMesh (Variables|Default|GetStage3))
  (Utilities|FlowControl|Delay (Variables|Default|GetGrowtime))
  (Variables|Default|SetStaticMesh (Variables|Default|GetCrop)))

(event Collision|EventActorBeginOverlap
  (params (OtherActor :type Actor%20Object%20Reference)))

(event EventTick
  (params (DeltaSeconds :type Float%20%28single-precision%29)))

(fn ConstructionScript)