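; House actor Blueprint with logic for gathering snow on its mesh during winter.
; BeginPlay caches the level's DayNight_Blueprint, and a SnowFall event drives the material's "Snow Amount" parameter from a timeline.
; The winter check that builds the dynamic SnowGather_M material and calls SnowFall is disconnected, so it never runs.
; That setup initializes "SnowAmount" without a space, unlike the timeline's parameter name.
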(event Custom|Snow%20Fall
  ;[0 0 0] Snow
  (bind _snow_amount (Timeline|Timeline_0 Play)
    (:Update
      (Rendering|Material|SetScalarParameterValue (Variables|Default|GetSnow%20Mat) "Snow Amount" _snow_amount :!class /Script/Engine.MaterialInstanceDynamic))))

(event EventBeginPlay
  (bind _outactors (Actor|GetAllActorsOfClass "/Game/Assets/Blueprints/DayNight_Blueprint.DayNight_Blueprint_C"))
  (Variables|Default|SetDayNight (Utilities|Array|Get(acopy) _outactors)))

(event Collision|EventActorBeginOverlap
  (params (OtherActor :type Actor%20Object%20Reference)))

(event EventTick
  (params (DeltaSeconds :type Float%20%28single-precision%29)))

(fn ConstructionScript)