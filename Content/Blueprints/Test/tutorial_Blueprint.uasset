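; VR tutorial guide actor that turns its Tut component toward the player camera every tick.
; BeginPlay creates a speech bubble widget, and Tick teleports the actor to FirstLocation while that widget's Move flag is true.
; A motion controller entering the Sphere sets Collided, which nothing in these graphs reads.
; A delayed text sequence about grabbing a hoe with the trigger is disconnected and never runs.
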(event OnComponentBeginOverlap(Sphere)
  (params (OverlappedComponent :type Primitive%20Component%20Object%20Reference) (OtherActor :type Actor%20Object%20Reference) (OtherComp :type Primitive%20Component%20Object%20Reference) (OtherBodyIndex :type Integer) (bFromSweep :type Boolean) (SweepResult :type Hit%20Result%20Structure%20%28by%20ref%29))
  (Utilities|Casting|CastToBP_MotionController OtherActor)
  (Variables|Default|SetCollided true))

(event EventBeginPlay
  (bind _returnvalue (UserInterface|CreateWidget "/Game/Widgets/Tutorial.Tutorial_C"))
  (Variables|Default|Setspeechbubble _returnvalue))

(event EventTick
  (params (DeltaSeconds :type Float%20%28single-precision%29))
  (bind _first_location (Variables|Default|Getfirst%20location))
  (Utilities|FlowControl|Sequence
    (:then_0
      (Transformation|SetWorldRotation (Variables|Default|Gettut) (Math|Rotator|FindLookatRotation (Transformation|GetWorldLocation (Variables|Default|Gettut)) (Camera|GetCameraLocation (Game|GetPlayerCameraManager 0))) false false))
    (:then_1
      (if (Variables|/Game/Widgets/Tutorial.Tutorial_C|GetMove (Variables|Default|Getspeechbubble))
        (Transformation|Teleport (Transformation|GetActorLocation _first_location) (Transformation|GetActorRotation _first_location))))))

(fn ConstructionScript)