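; Tree actor that reacts to the season reported by the level's DayNight_Blueprint, found on BeginPlay.
; Every Tick outside winter keeps the falling-leaves particles active.
; In winter it stops them and creates a fresh SnowGather_M dynamic material each frame with the tree's textures.
; A timeline then drives "Snow Amount" on that material, though the initial reset writes "SnowAmount" without a space.
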(event Custom|Snow%20Fall
  ;[0 0 0] Snow
  (bind _snow_amount (Timeline|Timeline_0 Play)
    (:Update
      (Rendering|Material|SetScalarParameterValue (Variables|Default|GetSnow%20Mat) "Snow Amount" _snow_amount :!class /Script/Engine.MaterialInstanceDynamic))))

(event EventBeginPlay
  (bind _outactors (Actor|GetAllActorsOfClass "/Game/Assets/Blueprints/DayNight_Blueprint.DayNight_Blueprint_C"))
  (Variables|Default|SetDayNight (Utilities|Array|Get(acopy) _outactors)))

(event Collision|EventActorBeginOverlap
  (params (OtherActor :type Actor%20Object%20Reference)))

(event EventTick
  (params (DeltaSeconds :type Float%20%28single-precision%29))
  ;[0 0 0] Snow
  (if (Variables|/Game/Assets/Blueprints/DayNight_Blueprint.DayNight_Blueprint_C|GetWinter (Variables|Default|GetDayNight))
    (Components|Activation|Deactivate (Variables|Default|GetFallingLeaves_P))
    (bind _returnvalue (Rendering|Material|CreateDynamicMaterialInstance "/Game/Weather/Snow/SnowGather_M.SnowGather_M" "None" :!class /Script/Engine.KismetMaterialLibrary))
    (Variables|Default|SetSnow%20Mat _returnvalue)
    (Rendering|Material|SetScalarParameterValue (Variables|Default|GetSnow%20Mat) "SnowAmount" 0.0 :!class /Script/Engine.MaterialInstanceDynamic)
    (Rendering|Material|SetTextureParameterValue (Variables|Default|GetSnow%20Mat) "Diffuse" "/Game/Textures/Tree/tree_uv_colour.tree_uv_colour")
    (Rendering|Material|SetTextureParameterValue (Variables|Default|GetSnow%20Mat) "Normal" "/Game/Textures/Tree/tree_uv_normal_map.tree_uv_normal_map")
    (Rendering|Material|SetMaterial (Variables|Debug|GetStaticMeshComponent) 0 (Variables|Default|GetSnow%20Mat))
    (CallFunction|SnowFall)
    (else
      (Components|Activation|Activate (Variables|Default|GetFallingLeaves_P) false))))

(fn ConstructionScript)