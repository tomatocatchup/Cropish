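; VR tutorial speech actor that moves between three preset locations as its stage flags are set.
; Overlap of a motion controller with its Sphere sets a Collided flag, and BeginPlay creates and stores a Tutorial widget.
; Tick turns the Sell component toward the player camera.
; Tick also polls First, Second and Third, which are not set here, using DoOnce to teleport once to each matching location actor.
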(event OnComponentBeginOverlap(Sphere)
  (params (OverlappedComponent :type Primitive%20Component%20Object%20Reference) (OtherActor :type Actor%20Object%20Reference) (OtherComp :type Primitive%20Component%20Object%20Reference) (OtherBodyIndex :type Integer) (bFromSweep :type Boolean) (SweepResult :type Hit%20Result%20Structure%20%28by%20ref%29))
  (Utilities|Casting|CastToBP_MotionController OtherActor)
  (Variables|Default|SetCollided true))

(event EventBeginPlay
  (bind _returnvalue (UserInterface|CreateWidget "/Game/Widgets/Tutorial.Tutorial_C"))
  (Variables|Default|SetTutorial _returnvalue))

(event EventTick
  (params (DeltaSeconds :type Float%20%28single-precision%29))
  (bind _third_location (Variables|Default|GetThird%20Location))
  (bind _first_location (Variables|Default|GetFirst%20Location))
  (bind _second_location (Variables|Default|GetSecond%20Location))
  (Utilities|FlowControl|Sequence
    (:then_0
      (Transformation|SetWorldRotation (Variables|Default|GetSell) (Math|Rotator|FindLookatRotation (Transformation|GetWorldLocation (Variables|Default|GetSell)) (Camera|GetCameraLocation (Game|GetPlayerCameraManager 0))) false false))
    (:then_1
      (Utilities|FlowControl|Sequence
        (:then_0
          (if (Variables|Default|Getfirst)
            (Utilities|FlowControl|DoOnce false
              (:Completed
                (Transformation|Teleport (Transformation|GetActorLocation _first_location) (Transformation|GetActorRotation _first_location))))))
        (:then_1
          (if (Variables|Default|Getsecond)
            (Utilities|FlowControl|DoOnce false
              (:Completed
                (Transformation|Teleport (Transformation|GetActorLocation _second_location) (Transformation|GetActorRotation _second_location))))))
        (:then_2
          (if (Variables|Default|Getthird)
            (Utilities|FlowControl|DoOnce false
              (:Completed
                (Transformation|Teleport (Transformation|GetActorLocation _third_location) (Transformation|GetActorRotation _third_location))))))))))

(fn ConstructionScript)