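; Button Blueprint that cycles a speed multiplier and shows the current value on its label.
; ButtonAction uses nested float comparisons to double SpeedMuliplier through fixed steps from 1 to 16, then wrap back to 1.
; Each change converts the value to text and sets it on the Name component.
; The multiplier is not applied to game speed in this graph, and the other events only call their parents or are disabled.
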(event EventBeginPlay
  (|CallParentFunction))

(event Collision|EventActorBeginOverlap
  (params (OtherActor :type Actor%20Object%20Reference))
  (|CallParentFunction OtherActor) ; This node is disabled and will not be called.\nDrag off pins to build functionality.
)

(event EventTick
  (params (DeltaSeconds :type Float%20%28single-precision%29))
  (|CallParentFunction DeltaSeconds))

(event EventButtonAction
  (Math|Float|CompareFloat (Variables|Default|GetSpeedMuliplier) 1.0
    (:>
      (Math|Float|CompareFloat (Variables|Default|GetSpeedMuliplier) 2.0
        (:>
          (Math|Float|CompareFloat (Variables|Default|GetSpeedMuliplier) 4.0
            (:>
              (Math|Float|CompareFloat (Variables|Default|GetSpeedMuliplier) 8.0
                (:>
                  (Math|Float|CompareFloat (Variables|Default|GetSpeedMuliplier) 16.0
                    (:==
                      (bind _output_get (Variables|Default|SetSpeedMuliplier 1.0))
                      (bind _output_get_2 (Variables|Default|SetNumberText (Utilities|Text|ToText(Float) _output_get "HalfToEven")))
                      (Rendering|Components|TextRender|SetText (Variables|Default|GetName) _output_get_2))))
                (:==
                  (bind _output_get_3 (Variables|Default|SetSpeedMuliplier 16.0))
                  (bind _output_get_4 (Variables|Default|SetNumberText (Utilities|Text|ToText(Float) _output_get_3 "HalfToEven")))
                  (Rendering|Components|TextRender|SetText (Variables|Default|GetName) _output_get_4))))
            (:==
              (bind _output_get_5 (Variables|Default|SetSpeedMuliplier 8.0))
              (bind _output_get_6 (Variables|Default|SetNumberText (Utilities|Text|ToText(Float) _output_get_5 "HalfToEven")))
              (Rendering|Components|TextRender|SetText (Variables|Default|GetName) _output_get_6))))
        (:==
          (bind _output_get_7 (Variables|Default|SetSpeedMuliplier 4.0))
          (bind _output_get_8 (Variables|Default|SetNumberText (Utilities|Text|ToText(Float) _output_get_7 "HalfToEven")))
          (Rendering|Components|TextRender|SetText (Variables|Default|GetName) _output_get_8))))
    (:==
      (bind _output_get_9 (Variables|Default|SetSpeedMuliplier 2.0))
      (bind _output_get_10 (Variables|Default|SetNumberText (Utilities|Text|ToText(Float) _output_get_9 "HalfToEven")))
      (Rendering|Components|TextRender|SetText (Variables|Default|GetName) _output_get_10))))

(fn ConstructionScript
  (|CallParentFunction))