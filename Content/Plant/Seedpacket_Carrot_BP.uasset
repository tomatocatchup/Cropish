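; Carrot seed packet that a motion controller can pick up and tip to pour seeds, showing its quantity as text on BeginPlay.
; Tick sets the Spawnseed flag while roll is between -120 and -60, using a DoOnce to start Plant playback once per tip and stopping it outside that range.
; Pickup disables physics and snaps the packet to the Items socket; Drop detaches it and restores physics.
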(event EventBeginPlay
  ;[1 1 1] Set the qty number
  (Rendering|Components|TextRender|SetText (Variables|Default|GetqtyNumber) (Utilities|Text|ToText(Integer) (Variables|Default|Getqty))))

(event EventPickup
  (params (AttachTo :type Scene%20Component%20Object%20Reference))
  ;[1 1 1] Will be changed when shop ui is implemented
  (Physics|SetSimulatePhysics (Variables|Debug|GetStaticMeshComponent) false)
  (bind _returnvalue (Transformation|AttachComponentToComponent (VehicleSound|GetRootComponent) AttachTo "Items" "SnapToTarget" "SnapToTarget" "KeepWorld" false))
  (Variables|Default|SetpickedUp _returnvalue))

(event EventDrop
  ;[1 1 1] Drop
  (Physics|SetSimulatePhysics (Variables|Debug|GetStaticMeshComponent) true)
  (Transformation|DetachFromActor "KeepWorld" "KeepWorld" "KeepWorld")
  (Variables|Default|SetpickedUp false))

(event EventTick
  (params (DeltaSeconds :type Float%20%28single-precision%29))
  (bind _returnvalue (Transformation|GetActorRotation))
  (bind _plant (Variables|Default|GetPlant))
  ;[1 1 1] Checks for rotation
  (Math|Float|CompareFloat (.roll _returnvalue) -6e+01
    (:>
      (Variables|Default|Setspawnseed false :!label _label)
      (Audio|Components|Audio|Stop _plant)
      (goto _label_3 Reset))
    (:==
      (Math|Float|CompareFloat (.roll _returnvalue) -1.2e+02 :!label _label_2
        (:>
          _)
        (:==
          _)
        (:<
          (goto _label))))
    (:<
      (goto _label_2)))
  (Variables|Default|Setspawnseed true)
  (Utilities|FlowControl|DoOnce false :!label _label_3
    (:Completed
      (Audio|Components|Audio|Play _plant 0.0))))

(fn ConstructionScript)