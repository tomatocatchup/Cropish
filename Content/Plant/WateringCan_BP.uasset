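; VR watering can actor that the motion controller can pick up and drop, pouring water when tilted.
; Pickup disables physics and snaps the can to the controller; Drop detaches it and restores physics.
; Tick checks actor roll: within a tilt range while held, it sets the Water flag and activates the Watering effect.
; A DoOnce starts the audio once per pour; otherwise effect and sound stop.
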(event EventBeginPlay
  (Components|Activation|Activate (Variables|Default|GetWatering) false))

(event Collision|EventActorBeginOverlap
  (params (OtherActor :type Actor%20Object%20Reference)))

(event EventPickup
  (params (AttachTo :type Scene%20Component%20Object%20Reference))
  (Physics|SetSimulatePhysics (Variables|Debug|GetStaticMeshComponent) false)
  (bind _returnvalue (Transformation|AttachComponentToComponent (VehicleSound|GetRootComponent) AttachTo "None" "SnapToTarget" "SnapToTarget" "KeepWorld" false))
  (Variables|Default|SetPicked%20Up _returnvalue))

(event EventTick
  (params (DeltaSeconds :type Float%20%28single-precision%29))
  (bind _returnvalue (Transformation|GetActorRotation))
  (bind _watering (Variables|Default|GetWatering))
  ;[0 0 0] Check rotation
  (Math|Float|CompareFloat (.roll _returnvalue) 1e+02
    (:>
      (Variables|Default|SetWater false :!label _label)
      (Components|Activation|Deactivate _watering)
      (Audio|Components|Audio|Stop (Variables|Default|Getwatering_audio))
      (goto _label_3 Reset))
    (:==
      (Math|Float|CompareFloat (.roll _returnvalue) 4e+01 :!label _label_2
        (:>
          _)
        (:==
          _)
        (:<
          (goto _label)))
      (if (Variables|Default|GetPicked%20Up)
        _
        (else
          (goto _label))))
    (:<
      (goto _label_2)))
  (bind _output_get (Variables|Default|SetWater true))
  (Components|Activation|Activate _watering _output_get)
  (Utilities|FlowControl|DoOnce false :!label _label_3
    (:Completed
      (Audio|Components|Audio|Play (Variables|Default|Getwatering_audio) 0.0))))

(event EventDrop
  (Physics|SetSimulatePhysics (Variables|Debug|GetStaticMeshComponent) true)
  (Transformation|DetachFromActor "KeepWorld" "KeepWorld" "KeepWorld")
  (Variables|Default|SetPicked%20Up false))

(fn ConstructionScript)